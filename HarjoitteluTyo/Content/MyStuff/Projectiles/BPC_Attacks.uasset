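; Attack component that provides area-of-effect abilities: delayed lightning strike, explosion and player heal.
; Each event spawns its AoE actor and binds to that actor's overlap dispatcher, so the component decides how damage or healing is applied through message calls.
; The heal line-traces from the target toward the ground to place its aura, and only heals that target when it overlaps.
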(event `AOELightningStrike`
  (params (`Spawn Transform Location` :type "Vector Structure") (DelayBeforeStrike :type "Float (single-precision)") (AttackTarget :type "Actor Object Reference") (IgnoreInstigator :type Boolean) (DrawDebugSphere :type Boolean) (Damage :type "Float (double-precision)") (Instigator :type "Pawn Object Reference"))
  ;[0 0 0] AOE Lightning Strike
  (bind _returnvalue (`|SpawnActorFromClass` "/Game/MyStuff/Projectiles/AoEStuff/Attacks/AoELightningDelayedStrike.AoELightningDelayedStrike_C" (`KismetMathLibrary.MakeTransform` `Spawn Transform Location`) "Undefined" "OverrideRootScale" null 256.0 DelayBeforeStrike AttackTarget IgnoreInstigator DrawDebugSphere false Damage Instigator))
  (add `/Game/MyStuff/Projectiles/AoEStuff/AoEBase.OnAOEOverlapActor` _returnvalue (`|CreateDelegate` :!event `AOEDamageTarget`)))

(event `AOEDamageTarget`
  (params (Actor :type "Actor Object Reference") (Damage :type "Float (double-precision)"))
  ;[0 0 0] Take Damage for AOE Attacks
  (message `/Game/MyStuff/DamageSystem/BPI_Damagable.TakeDamage` Actor (make `/Game/MyStuff/DamageSystem/S_DamageInfo` Damage "NewEnumerator3" "NewEnumerator1")))

(event `AOEExplosion`
  (params (`Spawn Transform Location` :type "Vector Structure") (IgnoreInstigator :type Boolean) (DrawDebugSphere :type Boolean) (TriggerOnSpawn :type Boolean) (Damage :type "Float (double-precision)") (Instigator :type "Pawn Object Reference"))
  ;[0 0 0] AOE Explosion
  (bind _returnvalue (`|SpawnActorFromClass` "/Game/MyStuff/Projectiles/AoEStuff/Attacks/AoEExplosion.AoEExplosion_C" (`KismetMathLibrary.MakeTransform` `Spawn Transform Location`) "Undefined" "OverrideRootScale" null IgnoreInstigator DrawDebugSphere TriggerOnSpawn Damage Instigator))
  (add `/Game/MyStuff/Projectiles/AoEStuff/AoEBase.OnAOEOverlapActor` _returnvalue (`|CreateDelegate` :!event `AOEDamageTarget`)))

(event `AOEHeal`
  (params (HealTarget :type "Actor Object Reference") (Damage :type "Float (double-precision)"))
  (bind _returnvalue (`Actor.K2_GetActorLocation` HealTarget))
  ;[0 0 0] AOEHeal
  (`/Engine/EditorBlueprintResources/StandardMacros.IsValid` HealTarget
    (:`Is Valid`
      (bind (_outhit _returnvalue_2) (`KismetSystemLibrary.LineTraceSingle` _returnvalue (* _returnvalue (1.0 1.0 -1000.0)) "TraceTypeQuery1" false (`|MakeArray` HealTarget)))
      (if _returnvalue_2
        (bind _returnvalue_3 (`|SpawnActorFromClass` "/Game/MyStuff/Projectiles/AoEStuff/Attacks/AoEPlayerHeal.AoEPlayerHeal_C" (`KismetMathLibrary.MakeTransform` (`.Location` (`GameplayStatics.BreakHitResult` _outhit))) "Undefined" "OverrideRootScale" null 0.2 5.0 "/Game/FXVarietyPack/Particles/P_ky_healAura.P_ky_healAura" 1.5 false false true Damage null))
        (add `/Game/MyStuff/Projectiles/AoEStuff/AoEBase.OnAOEOverlapActor` _returnvalue_3 (delegate `AOEHealEvent`))))))

(event `AOEHealEvent`
  (params (Actor :type "Actor Object Reference") (Damage :type "Float (double-precision)"))
  ;[0 0 0] AOEHeal
  (if (== Actor (stale `AOEHeal` HealTarget))
    (message `/Game/MyStuff/DamageSystem/BPI_Damagable.Heal` Actor Damage)))