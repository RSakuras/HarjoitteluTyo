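; Player attack component that spawns the basic attack and PowerShot projectiles.
; Each attack event passes owner, speed, gravity, homing settings, target and damage into its own projectile class, then binds to that projectile's impact dispatcher.
; A damage handler packs the amount into a damage info struct with fixed type and response, then sends it to the hit actor as a TakeDamage message.
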(event `BasicProjectile`
  (params (`Spawn Transform Location` :type "Vector Structure") (`Spawn Transform Rotation` :type "Rotator Structure") (Owner :type "Actor Object Reference") (Speed :type "Float (double-precision)") (Gravity :type "Float (double-precision)") (Target :type "Actor Object Reference") (IsHoming :type Boolean) (HomingAcceleration :type "Float (double-precision)") (Damage :type "Float (double-precision)"))
  ;[0 0 0] Basic Attack
  (bind _returnvalue (`|SpawnActorFromClass` "/Game/MyStuff/Projectiles/PlayerProjectiles/BP_Projectile_Player_BasicAttack.BP_Projectile_Player_BasicAttack_C" (`KismetMathLibrary.MakeTransform` `Spawn Transform Location` `Spawn Transform Rotation`) "Undefined" "OverrideRootScale" Owner Speed Gravity Target IsHoming HomingAcceleration Damage null))
  (add `/Game/MyStuff/Projectiles/BP_ProjectileBase.OnProjectileImpact` _returnvalue (`|CreateDelegate` :!event `ProjectileDamageTarget`)))

(event `ProjectileDamageTarget`
  (params (OtherActor :type "Actor Object Reference") (Hit :type "HitResult Structure") (Damage :type "Float (double-precision)"))
  ;[0 0 0] Take Damage
  (message `/Game/MyStuff/DamageSystem/BPI_Damagable.TakeDamage` OtherActor (make `/Game/MyStuff/DamageSystem/S_DamageInfo` Damage "NewEnumerator2" "NewEnumerator1")))

(event `PowerShot`
  (params (`Spawn Transform Location` :type "Vector Structure") (`Spawn Transform Rotation` :type "Rotator Structure") (Owner :type "Actor Object Reference") (Speed :type "Float (double-precision)") (Gravity :type "Float (double-precision)") (Target :type "Actor Object Reference") (IsHoming :type Boolean) (HomingAcceleration :type "Float (double-precision)") (Damage :type "Float (double-precision)"))
  ;[0 0 0] PowerShot
  (bind _returnvalue (`|SpawnActorFromClass` "/Game/MyStuff/Projectiles/PlayerProjectiles/BP_Projectile_Player_PowerShot.BP_Projectile_Player_PowerShot_C" (`KismetMathLibrary.MakeTransform` `Spawn Transform Location` `Spawn Transform Rotation`) "Undefined" "OverrideRootScale" Owner Speed Gravity Target IsHoming HomingAcceleration Damage null))
  (add `/Game/MyStuff/Projectiles/BP_ProjectileBase.OnProjectileImpact` _returnvalue (`|CreateDelegate` :!event `ProjectileDamageTarget`)))