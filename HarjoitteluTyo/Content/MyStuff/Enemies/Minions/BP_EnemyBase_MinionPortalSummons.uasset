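; Minion portal enemy that periodically summons minions and can be destroyed.
; On BeginPlay it sets up a health bar widget, spawns a first minion after a random delay, then starts a looping timer with a randomized interval.
; SpawnMinions places a randomly chosen standard or ranged minion at a navigable point nearby.
; On death it plays an impact effect, calls MinionSpawnerDestroyed and destroys itself.
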(event `self.ReceiveBeginPlay`
  (bind _returnvalue (`|CreateWidget` "/Game/MyStuff/DamageSystem/W_HealthBar.W_HealthBar_C" null self))
  (`WidgetComponent.SetWidget` (`self.HealthBar`) _returnvalue)
  (`KismetSystemLibrary.Delay` (`KismetMathLibrary.RandomFloatInRange` 1.0 10.0))
  (`self.SpawnMinions`)
  (`KismetSystemLibrary.K2_SetTimerDelegate` (`|CreateDelegate` :!event `SpawnMinions`) (`KismetMathLibrary.RandomFloatInRange` 15.0 25.0) true 1.0 0.5))

(event `SpawnMinions`
  ;[0 0 0] SpawnMinions
  (bind _randomlocation (`NavigationSystemV1.K2_GetRandomLocationInNavigableRadius` (`self.K2_GetActorLocation`) 350.0 null null))
  (`|SpawnActorFromClass` (select `int` (`KismetMathLibrary.RandomIntegerInRange` 0 1) :`0` "/Game/MyStuff/Enemies/Minions/EnemyBase_Minion.EnemyBase_Minion_C" :`1` "/Game/MyStuff/Enemies/Minions/EnemyBase_Minion_RangedVariant.EnemyBase_Minion_RangedVariant_C" :!type "Actor Class Reference") (`KismetMathLibrary.MakeTransform` _randomlocation) "AdjustIfPossibleButAlwaysSpawn" "OverrideRootScale" null null))

(event `self.OnDeath`
  ;[0 0 0] WhenDestroyed
  (`GameplayStatics.SpawnEmitterAtLocation` "/Game/InfinityBladeEffects/Effects/FX_Combat_Base/Impact/P_Impact_Enemy_IB.P_Impact_Enemy_IB" (`self.K2_GetActorLocation`) (struct :`Pitch` -90.0))
  (`self.MinionSpawnerDestroyed`)
  (`self.K2_DestroyActor`))

(fn `UserConstructionScript`
  (`parent.UserConstructionScript`))