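; BPC_ItemDataComponent is an actor component that makes its owner an inventory pickup, holding an item ID and quantity.
; On BeginPlay it turns on replication for the owning actor.
; Interactwith passes the ID's row name and quantity to the interacting player's inventory component, then destroys the owner if the add succeeds.
; LookAt is a stub that returns empty text.
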(event `self.ReceiveBeginPlay`
  (`Actor.SetReplicates` (`self.GetOwner`) true))

(event `/Game/MyStuff/Inventory/BPI_InteractInterface.InteractWith`
  (params (PlayerCharacter :type "/Game/TopDown/Blueprints/BP_TopDownCharacter Object Reference"))
  (bind _bpc_inventorysystem (`/Game/TopDown/Blueprints/BP_TopDownCharacter.BPC_InventorySystem` PlayerCharacter))
  (bind (_itemid_datatable _itemid_rowname) (break `DataTableRowHandle` (`self.ItemID`)))
  (`/Engine/EditorBlueprintResources/StandardMacros.IsValid` _bpc_inventorysystem
    (:`Is Valid`
      (bind _success (`/Game/MyStuff/Inventory/BPC_InventorySystem.AddToInventory` _bpc_inventorysystem _itemid_rowname (`self.Quantity`)))
      (if _success
        (`Actor.K2_DestroyActor` (`self.GetOwner`))))))

(fn `LookAt`
  (returns (Message :type Text))
  (return ""))